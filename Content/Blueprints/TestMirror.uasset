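; Virtual fitting mirror actor that dresses a Kinect-tracked user in clothing over the live camera feed.
; MotionSensor initialization supplies camera FOV, feed and depth textures, and selects V1 or V2 anim classes.
; Each tick compares sensor bones with the AvatarRaw skeleton to offset and width-scale avatar and garments, hiding clothes when tracking stops.
; Wearable events swap meshes and avatar occlusion masks; debug keys switch sensor, gender, avatar material, width and skeleton.
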(event Custom|AddCloth_Event
  (params (WearableData :type Wearable%20Data%20Structure))
  (bind (_displayname _skeletalmesh _targetcomponent _gender _category _thumbnailimage _fullbody _occlusionmap _longsleeved) (Utilities|Struct|BreakWearableData WearableData))
  (bind _motionsensor (Variables|Default|GetMotionSensor))
  ;[1 1 1] Add cloth
  (Class|SkinnedMeshComponent|SetSkeletalMesh _targetcomponent _skeletalmesh true)
  (CallFunction|SetOcclusionMap _targetcomponent _occlusionmap _fullbody)
  (if (Utilities|Enum|Equal(Enum) (Utilities|GetDisplayName (Variables|Default|GetTop)) (Utilities|GetDisplayName _targetcomponent))
    (if _longsleeved
      (Class|MotionSensorComponent|SetHandOcclusionMultiplier _motionsensor 0.7)
      (else
        (Class|MotionSensorComponent|SetHandOcclusionMultiplier _motionsensor 1.5)))))

(event Custom|RemoveCloth_Event
  (params (WearableData :type Wearable%20Data%20Structure))
  (bind (_displayname _skeletalmesh _targetcomponent _gender _category _thumbnailimage _fullbody) (Utilities|Struct|BreakWearableData WearableData))
  ;[1 1 1] Remove cloth
  (Class|SkinnedMeshComponent|SetSkeletalMesh _targetcomponent 0 true)
  (CallFunction|SetOcclusionMap _targetcomponent "/Game/Textures/White.White" _fullbody))

(event Custom|TrackingStart_Event
  (Development|PrintString "Tracking start")
  ;[1 1 1] Reset scale width offset
  (Variables|Default|SetScaleWidthOffset 0.0))

(event Custom|TrackingStop_Event
  (Development|PrintString "Tracking stop")
  ;[1 1 1] Reset scale width offset
  (Variables|Default|SetScaleWidthOffset 0.0))

(event Custom|GenderChange_Event
  (params (Gender :type Gender%20Enum :default "NewEnumerator0"))
  (bind _avataruser (Variables|Default|GetAvatarUser))
  (bind _top (Variables|Default|GetTop))
  (bind _avatarraw (Variables|Default|GetAvatarRaw))
  (bind _bottom (Variables|Default|GetBottom))
  (bind _avataruser_2 (Variables|Default|GetAvatarUser))
  ;[1 1 1] Change gender
  (switch Utilities|FlowControl|Switch|SwitchonGender Gender
    (:NewEnumerator0
      (bind _output_get (Variables|Default|SetGender "NewEnumerator0"))
      (Development|PrintString (Utilities|String|EnumtoString _output_get))
      (Class|SkinnedMeshComponent|SetSkeletalMesh _avataruser "/Game/AvatarMale/MaleFitA.MaleFitA" true)
      ;;[1 1 1] Default clothing (empty, use load cloth instead of this)
      (Class|SkinnedMeshComponent|SetSkeletalMesh _top 0 true)
      (Class|SkinnedMeshComponent|SetSkeletalMesh _bottom 0 true)
      (Class|SkinnedMeshComponent|SetSkeletalMesh _avatarraw "/Game/AvatarMale/MaleFitA.MaleFitA" true))
    (:NewEnumerator1
      (bind _output_get_2 (Variables|Default|SetGender "NewEnumerator1"))
      (Development|PrintString (Utilities|String|EnumtoString _output_get_2))
      (Class|SkinnedMeshComponent|SetSkeletalMesh _avataruser "/Game/AvatarFemale/FemaleFitA.FemaleFitA" true)
      (Class|SkinnedMeshComponent|SetSkeletalMesh _top 0 true)
      (Class|SkinnedMeshComponent|SetSkeletalMesh _bottom 0 true)
      (Class|SkinnedMeshComponent|SetSkeletalMesh _avatarraw "/Game/AvatarFemale/FemaleFitA.FemaleFitA" true)))
  (if (Variables|Default|GetIsShowAvatar)
    ;[1 1 1] Avatar ON/OFF
    (switch Utilities|FlowControl|Switch|SwitchonGender (Variables|Default|GetGender)
      (:NewEnumerator0
        (Rendering|Material|SetMaterial _avataruser_2 0 "/Game/AvatarMale/BodyMale.BodyMale"))
      (:NewEnumerator1
        (Rendering|Material|SetMaterial _avataruser_2 0 "/Game/AvatarFemale/BodyFemale.BodyFemale")))
    (Development|PrintString "Avatar  material changed")
    (Variables|Default|SetIsShowAvatar true)))

(event EventBeginPlay
  (bind _avataruser (Variables|Default|GetAvatarUser))
  (bind _top (Variables|Default|GetTop))
  (bind _avatarraw (Variables|Default|GetAvatarRaw))
  (bind _bottom (Variables|Default|GetBottom))
  (bind _motionsensor (Variables|Default|GetMotionSensor))
  (bind _avataruser_2 (Variables|Default|GetAvatarUser))
  (Input|EnableInput (Game|GetPlayerController 0))
  ;[1 1 1] Use cmd argument for sensor selection
  (Variables|Default|SetOverrideSensorType true)
  (Utilities|FlowControl|Sequence
    (:then_0
      ;[1 1 1] Init motion sensor
      (bind (_resx _resy _fov _widthmultiplier _returnvalue) (Class|MotionSensorComponent|Init (Variables|Default|GetMotionSensor) (Variables|Default|GetSensorType) (Variables|Default|GetOverrideSensorType)))
      ;;[1 1 1] Vertical FOV
      (Variables|Default|SetDefaultCameraFOV_Vertical _fov)
      (Variables|Default|SetSensorResX _resx)
      (Variables|Default|SetSensorResY _resy)
      (Variables|Default|SetWidthMultiplier _widthmultiplier)
      ;;[1 1 1] Could be changed with command line argument
      (Variables|Default|SetSensorType (Class|MotionSensorComponent|GetSensorType (Variables|Default|GetMotionSensor)))
      (switch Utilities|FlowControl|Switch|SwitchonESensorType (Variables|Default|GetSensorType)
        (:KINECT_V2
          ;;[1 1 1] Different value for every Kinect V2.0 sensor
          (Class|MotionSensorComponent|SetSensorOffset (Variables|Default|GetMotionSensor) "6.500000,0.000000,0.000000"))))
    (:then_1
      ;[1 1 1] Init video stream
      (if _returnvalue
        (bind _returnvalue_2 (Class|MotionSensorComponent|GetCameraFrame (Variables|Default|GetMotionSensor) "RGB"))
        (bind _returnvalue_3 (Class|MotionSensorComponent|GetCameraFrame (Variables|Default|GetMotionSensor) "USER"))
        (bind _returnvalue_4 (Class|MotionSensorComponent|CreateDynamicMaterialInstance (Variables|Default|GetMotionSensor) (Variables|Default|GetBackground) "/Game/Materials/BaseFeedScreenNoShadow.BaseFeedScreenNoShadow"))
        (Class|MotionSensorComponent|SetTextureParameterValue (Variables|Default|GetMotionSensor) _returnvalue_4 _returnvalue_2 "Color")
        (Class|MotionSensorComponent|SetTextureParameterValue (Variables|Default|GetMotionSensor) _returnvalue_4 _returnvalue_3 "NoMask")
        (Rendering|Material|SetScalarParameterValue _returnvalue_4 "CamResX" (Math|Conversions|ToFloat(Integer) (Variables|Default|GetSensorResX)) :!class /Script/Engine.MaterialInstanceDynamic)
        (Rendering|Material|SetScalarParameterValue _returnvalue_4 "CamResY" (Math|Conversions|ToFloat(Integer) (Variables|Default|GetSensorResY)) :!class /Script/Engine.MaterialInstanceDynamic)
        (bind _returnvalue_5 (Class|MotionSensorComponent|CreateDynamicMaterialInstanceSkeletal (Variables|Default|GetMotionSensor) (Variables|Default|GetAvatarUser) "/Game/Materials/Avatar.Avatar"))
        (Class|MotionSensorComponent|SetTextureParameterValue (Variables|Default|GetMotionSensor) _returnvalue_5 _returnvalue_2 "Color")
        (Class|MotionSensorComponent|SetTextureParameterValue (Variables|Default|GetMotionSensor) _returnvalue_5 "/Game/Textures/black.Black" "MaskTop")
        (Rendering|Material|SetScalarParameterValue _returnvalue_5 "CamResX" (Math|Conversions|ToFloat(Integer) (Variables|Default|GetSensorResX)) :!class /Script/Engine.MaterialInstanceDynamic)
        (Rendering|Material|SetScalarParameterValue _returnvalue_5 "CamResY" (Math|Conversions|ToFloat(Integer) (Variables|Default|GetSensorResY)) :!class /Script/Engine.MaterialInstanceDynamic)
        ;[1 1 1] User preview
        (Utilities|FlowControl|Delay 0.2)
        (bind _returnvalue_6 (Appearance|GetDynamicMaterial (Variables|/Game/UI/MainUI.MainUI_C|GetUserPreview (Variables|Default|GetUI)) :!class /Script/UMG.Image))
        (bind _returnvalue_7 (Class|MotionSensorComponent|GetCameraFrame (Variables|Default|GetMotionSensor) "USER"))
        (Rendering|Material|SetTextureParameterValue _returnvalue_6 "Color" _returnvalue_7)))
    (:then_2
      ;[1 1 1] Change gender
      (switch Utilities|FlowControl|Switch|SwitchonGender (Variables|Default|GetGender)
        (:NewEnumerator0
          (bind _output_get (Variables|Default|SetGender "NewEnumerator0"))
          (Development|PrintString (Utilities|String|EnumtoString _output_get))
          (Class|SkinnedMeshComponent|SetSkeletalMesh _avataruser "/Game/AvatarMale/MaleFitA.MaleFitA" true)
          ;;[1 1 1] Default clothing (empty, use load cloth instead of this)
          (Class|SkinnedMeshComponent|SetSkeletalMesh _top 0 true)
          (Class|SkinnedMeshComponent|SetSkeletalMesh _bottom 0 true)
          (Class|SkinnedMeshComponent|SetSkeletalMesh _avatarraw "/Game/AvatarMale/MaleFitA.MaleFitA" true))
        (:NewEnumerator1
          (bind _output_get_2 (Variables|Default|SetGender "NewEnumerator1"))
          (Development|PrintString (Utilities|String|EnumtoString _output_get_2))
          (Class|SkinnedMeshComponent|SetSkeletalMesh _avataruser "/Game/AvatarFemale/FemaleFitA.FemaleFitA" true)
          (Class|SkinnedMeshComponent|SetSkeletalMesh _top 0 true)
          (Class|SkinnedMeshComponent|SetSkeletalMesh _bottom 0 true)
          (Class|SkinnedMeshComponent|SetSkeletalMesh _avatarraw "/Game/AvatarFemale/FemaleFitA.FemaleFitA" true)))
      (if (Variables|Default|GetIsShowAvatar)
        ;[1 1 1] Avatar ON/OFF
        (switch Utilities|FlowControl|Switch|SwitchonGender (Variables|Default|GetGender)
          (:NewEnumerator0
            (Rendering|Material|SetMaterial _avataruser_2 0 "/Game/AvatarMale/BodyMale.BodyMale"))
          (:NewEnumerator1
            (Rendering|Material|SetMaterial _avataruser_2 0 "/Game/AvatarFemale/BodyFemale.BodyFemale")))
        (Development|PrintString "Avatar  material changed")
        (Variables|Default|SetIsShowAvatar true)))
    (:then_3
      (if _returnvalue
        (Utilities|FlowControl|Sequence
          (:then_0
            (bind _returnvalue_8 (Class|MotionSensorComponent|CreateDynamicMaterialInstance _motionsensor (Variables|Default|GetForeGround) "/Game/Materials/DepthPreview.DepthPreview")))
          (:then_1
            (bind _returnvalue_9 (Class|MotionSensorComponent|GetCameraFrame _motionsensor "USER")))
          (:then_2
            (bind _returnvalue_10 (Class|MotionSensorComponent|GetCameraFrame _motionsensor "DEPTH"))
            (Class|MotionSensorComponent|SetTextureParameterValue (Variables|Default|GetMotionSensor) _returnvalue_8 _returnvalue_2 "Color")
            (Class|MotionSensorComponent|SetTextureParameterValue (Variables|Default|GetMotionSensor) _returnvalue_8 _returnvalue_9 "User")
            (Class|MotionSensorComponent|SetTextureParameterValue (Variables|Default|GetMotionSensor) _returnvalue_8 _returnvalue_10 "DepthKinect")
            (Rendering|Material|SetScalarParameterValue _returnvalue_8 "CamResX" (Math|Conversions|ToFloat(Integer) (Variables|Default|GetSensorResX)) :!class /Script/Engine.MaterialInstanceDynamic)
            (Rendering|Material|SetScalarParameterValue _returnvalue_8 "CamResY" (Math|Conversions|ToFloat(Integer) (Variables|Default|GetSensorResY)) :!class /Script/Engine.MaterialInstanceDynamic)))))
    (:then_4
      ;[1 1 1] Set main camera
      (Game|Player|SetViewTargetwithBlend (Game|GetPlayerController 0) self 0.0 "VTBlend_Linear" 0.0 false))
    (:then_5
      ;[1 1 1] Set Anim instance
      (switch Utilities|FlowControl|Switch|SwitchonESensorType (Variables|Default|GetSensorType)
        (:KINECT_V1
          (Class|SkeletalMeshComponent|SetAnimClass (Variables|Default|GetTop) "/Game/AvatarMale/K1AnimBlueprint.K1AnimBlueprint_C")
          (Class|SkeletalMeshComponent|SetAnimClass (Variables|Default|GetAvatarRaw) "/Game/AvatarMale/K1AnimBlueprintRaw.K1AnimBlueprintRaw_C"))
        (:KINECT_V2
          (Class|SkeletalMeshComponent|SetAnimClass (Variables|Default|GetTop) "/Game/AvatarMale/K2AnimBlueprint.K2AnimBlueprint_C")
          (Class|SkeletalMeshComponent|SetAnimClass (Variables|Default|GetAvatarRaw) "/Game/AvatarMale/K2AnimBlueprintRaw.K2AnimBlueprintRaw_C"))))))

(event EventEndPlay
  (params (EndPlayReason :type EEndPlayReason%20Enum :default "Destroyed"))
  ;[1 1 1] Cleanup
  (Class|MotionSensorComponent|Cleanup (Variables|Default|GetMotionSensor)))

(event EventTick
  (params (DeltaSeconds :type Float%20%28single-precision%29))
  (bind _returnvalue (Game|GetPlayerController 0))
  (bind _top (Variables|Default|GetTop))
  (bind _istracking (Variables|Default|GetIsTracking))
  (bind _sensorresx (Variables|Default|GetSensorResX))
  (bind _sensorresy (Variables|Default|GetSensorResY))
  (bind _returnvalue_2 (Math|Conversions|ToFloat(Integer) _sensorresx))
  (bind _returnvalue_3 (Math|Conversions|ToFloat(Integer) _sensorresy))
  (bind (_sizex _sizey) (HUD|GetViewportSize _returnvalue))
  (bind _returnvalue_4 (/ _returnvalue_2 _returnvalue_3))
  (bind _returnvalue_5 (Math|Conversions|ToFloat(Integer) _sizex))
  (bind _returnvalue_6 (Math|Conversions|ToFloat(Integer) _sizey))
  (bind _returnvalue_7 (/ _returnvalue_5 _returnvalue_6))
  (Utilities|FlowControl|Sequence
    (:then_0
      ;[1 1 1] Camera FOV
      (bind _output_get (Variables|/Script/Engine.CameraComponent|SetAspectRatio (Variables|Default|GetCameraComponent) _returnvalue_7))
      (if (>= _returnvalue_4 _output_get)
        (Variables|/Script/Engine.CameraComponent|SetFieldOfView (Variables|Default|GetCameraComponent) (* (Class|KismetMathLibrary|DegAtan (* _returnvalue_7 (Math|Trig|Tan(Degrees) (/ (Variables|Default|GetDefaultCameraFOV_Vertical) 2.0)))) 2.0))
        (else
          (Variables|/Script/Engine.CameraComponent|SetFieldOfView (Variables|Default|GetCameraComponent) (* (Class|KismetMathLibrary|DegAtan (* _returnvalue_4 (Math|Trig|Tan(Degrees) (/ (Variables|Default|GetDefaultCameraFOV_Vertical) 2.0)))) 2.0)))))
    (:then_1
      ;[1 1 1] Avatar skeleton offsets
      (if (Class|MotionSensorComponent|IsTracking (Variables|Default|GetMotionSensor))
        (bind (_offsetvectorhip _offsetvectorneck) (CallFunction|GetBodyOffset false))
        (Utilities|FlowControl|Sequence
          (:then_0
            (CallFunction|SetAnimOffset (Variables|Default|GetTop) _offsetvectorhip _offsetvectorneck (Variables|Default|GetScaleWidth)))
          (:then_1
            (CallFunction|SetAnimOffset (Variables|Default|GetAvatarUser) _offsetvectorhip _offsetvectorneck (Variables|Default|GetScaleWidth)))
          (:then_2
            (CallFunction|SetAnimOffset (Variables|Default|GetBottom) _offsetvectorhip _offsetvectorneck (Variables|Default|GetScaleWidth))))))
    (:then_2
      ;[1 1 1] Body Scale
      (if (Class|MotionSensorComponent|IsTracking (Variables|Default|GetMotionSensor))
        (bind (_scaleshoulder _scalehip) (CallFunction|GetBodyScale))
        (Variables|Default|SetScaleWidth (+ (* (/ (+ _scaleshoulder _scalehip) 2.0) (Variables|Default|GetWidthMultiplier)) (Variables|Default|GetScaleWidthOffset)))))
    (:then_3
      ;[1 1 1] Draw debug skeleton if enabled
      (if (Variables|Default|GetDebugSkeleton)
        (CallFunction|DrawDebugSkeleton 2.0 "(R=0.000000,G=1.000000,B=1.000000,A=1.000000)")))
    (:then_4
      ;[1 1 1] Show hide based on angle (Kinect v2,0)
      (Utilities|FlowControl|Sequence
        (:then_0
          (if (Math|Boolean|ANDBoolean (> (Math|Float|Absolute(Float) (- (.Roll (Math|Rotator|BreakRotator (Class|MotionSensorComponent|GetBoneRotation (Variables|Default|GetMotionSensor) "SpineBase"))) 9e+01)) 9e+01) (Utilities|Enum|Equal(Enum) (Variables|Default|GetSensorType) "KINECT_V2") (Variables|Default|GetIsTracking))
            (if (and _istracking (Variables|/Script/Engine.SceneComponent|GetbVisible (Variables|Default|GetTop)))
              (Default|DisplayMessage (Variables|/Game/UI/MainUI.MainUI_C|GetNotification (Variables|Default|GetUI)) "Face to the camera please!" 1)
              (Rendering|SetVisibility _top false false :!label _label))
            (else
              (Rendering|SetVisibility _top true false))))
        (:then_1
          (if (not _istracking)
            (goto _label)))))))

(event Input|KeyboardEvents|R
  (params (Key :type Key%20Structure))
  (bind _avataruser (Variables|Default|GetAvatarUser))
  (bind _top (Variables|Default|GetTop))
  (bind _avatarraw (Variables|Default|GetAvatarRaw))
  (bind _bottom (Variables|Default|GetBottom))
  (bind _motionsensor (Variables|Default|GetMotionSensor))
  (bind _avataruser_2 (Variables|Default|GetAvatarUser))
  ;[1 1 1] Restart sensor
  (:Pressed
    ;[1 1 1] Switch between sensors
    (Utilities|FlowControl|Sequence
      (:then_0
        (Class|MotionSensorComponent|Cleanup (Variables|Default|GetMotionSensor)))
      (:then_1
        (Variables|Default|SetOverrideSensorType false))
      (:then_2
        (Utilities|FlowControl|Sequence
          (:then_0
            ;[1 1 1] Init motion sensor
            (bind (_resx _resy _fov _widthmultiplier _returnvalue) (Class|MotionSensorComponent|Init (Variables|Default|GetMotionSensor) (Variables|Default|GetSensorType) (Variables|Default|GetOverrideSensorType)))
            ;;[1 1 1] Vertical FOV
            (Variables|Default|SetDefaultCameraFOV_Vertical _fov)
            (Variables|Default|SetSensorResX _resx)
            (Variables|Default|SetSensorResY _resy)
            (Variables|Default|SetWidthMultiplier _widthmultiplier)
            ;;[1 1 1] Could be changed with command line argument
            (Variables|Default|SetSensorType (Class|MotionSensorComponent|GetSensorType (Variables|Default|GetMotionSensor)))
            (switch Utilities|FlowControl|Switch|SwitchonESensorType (Variables|Default|GetSensorType)
              (:KINECT_V2
                ;;[1 1 1] Different value for every Kinect V2.0 sensor
                (Class|MotionSensorComponent|SetSensorOffset (Variables|Default|GetMotionSensor) "6.500000,0.000000,0.000000"))))
          (:then_1
            ;[1 1 1] Init video stream
            (if _returnvalue
              (bind _returnvalue_2 (Class|MotionSensorComponent|GetCameraFrame (Variables|Default|GetMotionSensor) "RGB"))
              (bind _returnvalue_3 (Class|MotionSensorComponent|GetCameraFrame (Variables|Default|GetMotionSensor) "USER"))
              (bind _returnvalue_4 (Class|MotionSensorComponent|CreateDynamicMaterialInstance (Variables|Default|GetMotionSensor) (Variables|Default|GetBackground) "/Game/Materials/BaseFeedScreenNoShadow.BaseFeedScreenNoShadow"))
              (Class|MotionSensorComponent|SetTextureParameterValue (Variables|Default|GetMotionSensor) _returnvalue_4 _returnvalue_2 "Color")
              (Class|MotionSensorComponent|SetTextureParameterValue (Variables|Default|GetMotionSensor) _returnvalue_4 _returnvalue_3 "NoMask")
              (Rendering|Material|SetScalarParameterValue _returnvalue_4 "CamResX" (Math|Conversions|ToFloat(Integer) (Variables|Default|GetSensorResX)) :!class /Script/Engine.MaterialInstanceDynamic)
              (Rendering|Material|SetScalarParameterValue _returnvalue_4 "CamResY" (Math|Conversions|ToFloat(Integer) (Variables|Default|GetSensorResY)) :!class /Script/Engine.MaterialInstanceDynamic)
              (bind _returnvalue_5 (Class|MotionSensorComponent|CreateDynamicMaterialInstanceSkeletal (Variables|Default|GetMotionSensor) (Variables|Default|GetAvatarUser) "/Game/Materials/Avatar.Avatar"))
              (Class|MotionSensorComponent|SetTextureParameterValue (Variables|Default|GetMotionSensor) _returnvalue_5 _returnvalue_2 "Color")
              (Class|MotionSensorComponent|SetTextureParameterValue (Variables|Default|GetMotionSensor) _returnvalue_5 "/Game/Textures/black.Black" "MaskTop")
              (Rendering|Material|SetScalarParameterValue _returnvalue_5 "CamResX" (Math|Conversions|ToFloat(Integer) (Variables|Default|GetSensorResX)) :!class /Script/Engine.MaterialInstanceDynamic)
              (Rendering|Material|SetScalarParameterValue _returnvalue_5 "CamResY" (Math|Conversions|ToFloat(Integer) (Variables|Default|GetSensorResY)) :!class /Script/Engine.MaterialInstanceDynamic)
              ;[1 1 1] User preview
              (Utilities|FlowControl|Delay 0.2)
              (bind _returnvalue_6 (Appearance|GetDynamicMaterial (Variables|/Game/UI/MainUI.MainUI_C|GetUserPreview (Variables|Default|GetUI)) :!class /Script/UMG.Image))
              (bind _returnvalue_7 (Class|MotionSensorComponent|GetCameraFrame (Variables|Default|GetMotionSensor) "USER"))
              (Rendering|Material|SetTextureParameterValue _returnvalue_6 "Color" _returnvalue_7)))
          (:then_2
            ;[1 1 1] Change gender
            (switch Utilities|FlowControl|Switch|SwitchonGender (Variables|Default|GetGender)
              (:NewEnumerator0
                (bind _output_get (Variables|Default|SetGender "NewEnumerator0"))
                (Development|PrintString (Utilities|String|EnumtoString _output_get))
                (Class|SkinnedMeshComponent|SetSkeletalMesh _avataruser "/Game/AvatarMale/MaleFitA.MaleFitA" true)
                ;;[1 1 1] Default clothing (empty, use load cloth instead of this)
                (Class|SkinnedMeshComponent|SetSkeletalMesh _top 0 true)
                (Class|SkinnedMeshComponent|SetSkeletalMesh _bottom 0 true)
                (Class|SkinnedMeshComponent|SetSkeletalMesh _avatarraw "/Game/AvatarMale/MaleFitA.MaleFitA" true))
              (:NewEnumerator1
                (bind _output_get_2 (Variables|Default|SetGender "NewEnumerator1"))
                (Development|PrintString (Utilities|String|EnumtoString _output_get_2))
                (Class|SkinnedMeshComponent|SetSkeletalMesh _avataruser "/Game/AvatarFemale/FemaleFitA.FemaleFitA" true)
                (Class|SkinnedMeshComponent|SetSkeletalMesh _top 0 true)
                (Class|SkinnedMeshComponent|SetSkeletalMesh _bottom 0 true)
                (Class|SkinnedMeshComponent|SetSkeletalMesh _avatarraw "/Game/AvatarFemale/FemaleFitA.FemaleFitA" true)))
            (if (Variables|Default|GetIsShowAvatar)
              ;[1 1 1] Avatar ON/OFF
              (switch Utilities|FlowControl|Switch|SwitchonGender (Variables|Default|GetGender)
                (:NewEnumerator0
                  (Rendering|Material|SetMaterial _avataruser_2 0 "/Game/AvatarMale/BodyMale.BodyMale"))
                (:NewEnumerator1
                  (Rendering|Material|SetMaterial _avataruser_2 0 "/Game/AvatarFemale/BodyFemale.BodyFemale")))
              (Development|PrintString "Avatar  material changed")
              (Variables|Default|SetIsShowAvatar true)))
          (:then_3
            (if _returnvalue
              (Utilities|FlowControl|Sequence
                (:then_0
                  (bind _returnvalue_8 (Class|MotionSensorComponent|CreateDynamicMaterialInstance _motionsensor (Variables|Default|GetForeGround) "/Game/Materials/DepthPreview.DepthPreview")))
                (:then_1
                  (bind _returnvalue_9 (Class|MotionSensorComponent|GetCameraFrame _motionsensor "USER")))
                (:then_2
                  (bind _returnvalue_10 (Class|MotionSensorComponent|GetCameraFrame _motionsensor "DEPTH"))
                  (Class|MotionSensorComponent|SetTextureParameterValue (Variables|Default|GetMotionSensor) _returnvalue_8 _returnvalue_2 "Color")
                  (Class|MotionSensorComponent|SetTextureParameterValue (Variables|Default|GetMotionSensor) _returnvalue_8 _returnvalue_9 "User")
                  (Class|MotionSensorComponent|SetTextureParameterValue (Variables|Default|GetMotionSensor) _returnvalue_8 _returnvalue_10 "DepthKinect")
                  (Rendering|Material|SetScalarParameterValue _returnvalue_8 "CamResX" (Math|Conversions|ToFloat(Integer) (Variables|Default|GetSensorResX)) :!class /Script/Engine.MaterialInstanceDynamic)
                  (Rendering|Material|SetScalarParameterValue _returnvalue_8 "CamResY" (Math|Conversions|ToFloat(Integer) (Variables|Default|GetSensorResY)) :!class /Script/Engine.MaterialInstanceDynamic)))))
          (:then_4
            ;[1 1 1] Set main camera
            (Game|Player|SetViewTargetwithBlend (Game|GetPlayerController 0) self 0.0 "VTBlend_Linear" 0.0 false))
          (:then_5
            ;[1 1 1] Set Anim instance
            (switch Utilities|FlowControl|Switch|SwitchonESensorType (Variables|Default|GetSensorType)
              (:KINECT_V1
                (Class|SkeletalMeshComponent|SetAnimClass (Variables|Default|GetTop) "/Game/AvatarMale/K1AnimBlueprint.K1AnimBlueprint_C")
                (Class|SkeletalMeshComponent|SetAnimClass (Variables|Default|GetAvatarRaw) "/Game/AvatarMale/K1AnimBlueprintRaw.K1AnimBlueprintRaw_C"))
              (:KINECT_V2
                (Class|SkeletalMeshComponent|SetAnimClass (Variables|Default|GetTop) "/Game/AvatarMale/K2AnimBlueprint.K2AnimBlueprint_C")
                (Class|SkeletalMeshComponent|SetAnimClass (Variables|Default|GetAvatarRaw) "/Game/AvatarMale/K2AnimBlueprintRaw.K2AnimBlueprintRaw_C")))))))))

(event Input|KeyboardEvents|D
  (params (Key :type Key%20Structure))
  ;[1 1 1] Debug SKELETON ON/OFF
  (:Pressed
    (Variables|Default|SetDebugSkeleton (not (Variables|Default|GetDebugSkeleton)))))

(event Input|KeyboardEvents|1
  (params (Key :type Key%20Structure))
  (bind _avataruser (Variables|Default|GetAvatarUser))
  (bind _top (Variables|Default|GetTop))
  (bind _avatarraw (Variables|Default|GetAvatarRaw))
  (bind _bottom (Variables|Default|GetBottom))
  (bind _motionsensor (Variables|Default|GetMotionSensor))
  (bind _avataruser_2 (Variables|Default|GetAvatarUser))
  ;[1 1 1] Switch between sensors
  (:Pressed
    (Development|ExecuteConsoleCommand "r.setRes 960x720" (Game|GetPlayerController 0))
    (Variables|Default|SetSensorType "KINECT_V1")
    (Utilities|FlowControl|Sequence
      (:then_0
        (Class|MotionSensorComponent|Cleanup (Variables|Default|GetMotionSensor)))
      (:then_1
        (Variables|Default|SetOverrideSensorType false))
      (:then_2
        (Utilities|FlowControl|Sequence
          (:then_0
            ;[1 1 1] Init motion sensor
            (bind (_resx _resy _fov _widthmultiplier _returnvalue) (Class|MotionSensorComponent|Init (Variables|Default|GetMotionSensor) (Variables|Default|GetSensorType) (Variables|Default|GetOverrideSensorType)))
            ;;[1 1 1] Vertical FOV
            (Variables|Default|SetDefaultCameraFOV_Vertical _fov)
            (Variables|Default|SetSensorResX _resx)
            (Variables|Default|SetSensorResY _resy)
            (Variables|Default|SetWidthMultiplier _widthmultiplier)
            ;;[1 1 1] Could be changed with command line argument
            (Variables|Default|SetSensorType (Class|MotionSensorComponent|GetSensorType (Variables|Default|GetMotionSensor)))
            (switch Utilities|FlowControl|Switch|SwitchonESensorType (Variables|Default|GetSensorType)
              (:KINECT_V2
                ;;[1 1 1] Different value for every Kinect V2.0 sensor
                (Class|MotionSensorComponent|SetSensorOffset (Variables|Default|GetMotionSensor) "6.500000,0.000000,0.000000"))))
          (:then_1
            ;[1 1 1] Init video stream
            (if _returnvalue
              (bind _returnvalue_2 (Class|MotionSensorComponent|GetCameraFrame (Variables|Default|GetMotionSensor) "RGB"))
              (bind _returnvalue_3 (Class|MotionSensorComponent|GetCameraFrame (Variables|Default|GetMotionSensor) "USER"))
              (bind _returnvalue_4 (Class|MotionSensorComponent|CreateDynamicMaterialInstance (Variables|Default|GetMotionSensor) (Variables|Default|GetBackground) "/Game/Materials/BaseFeedScreenNoShadow.BaseFeedScreenNoShadow"))
              (Class|MotionSensorComponent|SetTextureParameterValue (Variables|Default|GetMotionSensor) _returnvalue_4 _returnvalue_2 "Color")
              (Class|MotionSensorComponent|SetTextureParameterValue (Variables|Default|GetMotionSensor) _returnvalue_4 _returnvalue_3 "NoMask")
              (Rendering|Material|SetScalarParameterValue _returnvalue_4 "CamResX" (Math|Conversions|ToFloat(Integer) (Variables|Default|GetSensorResX)) :!class /Script/Engine.MaterialInstanceDynamic)
              (Rendering|Material|SetScalarParameterValue _returnvalue_4 "CamResY" (Math|Conversions|ToFloat(Integer) (Variables|Default|GetSensorResY)) :!class /Script/Engine.MaterialInstanceDynamic)
              (bind _returnvalue_5 (Class|MotionSensorComponent|CreateDynamicMaterialInstanceSkeletal (Variables|Default|GetMotionSensor) (Variables|Default|GetAvatarUser) "/Game/Materials/Avatar.Avatar"))
              (Class|MotionSensorComponent|SetTextureParameterValue (Variables|Default|GetMotionSensor) _returnvalue_5 _returnvalue_2 "Color")
              (Class|MotionSensorComponent|SetTextureParameterValue (Variables|Default|GetMotionSensor) _returnvalue_5 "/Game/Textures/black.Black" "MaskTop")
              (Rendering|Material|SetScalarParameterValue _returnvalue_5 "CamResX" (Math|Conversions|ToFloat(Integer) (Variables|Default|GetSensorResX)) :!class /Script/Engine.MaterialInstanceDynamic)
              (Rendering|Material|SetScalarParameterValue _returnvalue_5 "CamResY" (Math|Conversions|ToFloat(Integer) (Variables|Default|GetSensorResY)) :!class /Script/Engine.MaterialInstanceDynamic)
              ;[1 1 1] User preview
              (Utilities|FlowControl|Delay 0.2)
              (bind _returnvalue_6 (Appearance|GetDynamicMaterial (Variables|/Game/UI/MainUI.MainUI_C|GetUserPreview (Variables|Default|GetUI)) :!class /Script/UMG.Image))
              (bind _returnvalue_7 (Class|MotionSensorComponent|GetCameraFrame (Variables|Default|GetMotionSensor) "USER"))
              (Rendering|Material|SetTextureParameterValue _returnvalue_6 "Color" _returnvalue_7)))
          (:then_2
            ;[1 1 1] Change gender
            (switch Utilities|FlowControl|Switch|SwitchonGender (Variables|Default|GetGender)
              (:NewEnumerator0
                (bind _output_get (Variables|Default|SetGender "NewEnumerator0"))
                (Development|PrintString (Utilities|String|EnumtoString _output_get))
                (Class|SkinnedMeshComponent|SetSkeletalMesh _avataruser "/Game/AvatarMale/MaleFitA.MaleFitA" true)
                ;;[1 1 1] Default clothing (empty, use load cloth instead of this)
                (Class|SkinnedMeshComponent|SetSkeletalMesh _top 0 true)
                (Class|SkinnedMeshComponent|SetSkeletalMesh _bottom 0 true)
                (Class|SkinnedMeshComponent|SetSkeletalMesh _avatarraw "/Game/AvatarMale/MaleFitA.MaleFitA" true))
              (:NewEnumerator1
                (bind _output_get_2 (Variables|Default|SetGender "NewEnumerator1"))
                (Development|PrintString (Utilities|String|EnumtoString _output_get_2))
                (Class|SkinnedMeshComponent|SetSkeletalMesh _avataruser "/Game/AvatarFemale/FemaleFitA.FemaleFitA" true)
                (Class|SkinnedMeshComponent|SetSkeletalMesh _top 0 true)
                (Class|SkinnedMeshComponent|SetSkeletalMesh _bottom 0 true)
                (Class|SkinnedMeshComponent|SetSkeletalMesh _avatarraw "/Game/AvatarFemale/FemaleFitA.FemaleFitA" true)))
            (if (Variables|Default|GetIsShowAvatar)
              ;[1 1 1] Avatar ON/OFF
              (switch Utilities|FlowControl|Switch|SwitchonGender (Variables|Default|GetGender)
                (:NewEnumerator0
                  (Rendering|Material|SetMaterial _avataruser_2 0 "/Game/AvatarMale/BodyMale.BodyMale"))
                (:NewEnumerator1
                  (Rendering|Material|SetMaterial _avataruser_2 0 "/Game/AvatarFemale/BodyFemale.BodyFemale")))
              (Development|PrintString "Avatar  material changed")
              (Variables|Default|SetIsShowAvatar true)))
          (:then_3
            (if _returnvalue
              (Utilities|FlowControl|Sequence
                (:then_0
                  (bind _returnvalue_8 (Class|MotionSensorComponent|CreateDynamicMaterialInstance _motionsensor (Variables|Default|GetForeGround) "/Game/Materials/DepthPreview.DepthPreview")))
                (:then_1
                  (bind _returnvalue_9 (Class|MotionSensorComponent|GetCameraFrame _motionsensor "USER")))
                (:then_2
                  (bind _returnvalue_10 (Class|MotionSensorComponent|GetCameraFrame _motionsensor "DEPTH"))
                  (Class|MotionSensorComponent|SetTextureParameterValue (Variables|Default|GetMotionSensor) _returnvalue_8 _returnvalue_2 "Color")
                  (Class|MotionSensorComponent|SetTextureParameterValue (Variables|Default|GetMotionSensor) _returnvalue_8 _returnvalue_9 "User")
                  (Class|MotionSensorComponent|SetTextureParameterValue (Variables|Default|GetMotionSensor) _returnvalue_8 _returnvalue_10 "DepthKinect")
                  (Rendering|Material|SetScalarParameterValue _returnvalue_8 "CamResX" (Math|Conversions|ToFloat(Integer) (Variables|Default|GetSensorResX)) :!class /Script/Engine.MaterialInstanceDynamic)
                  (Rendering|Material|SetScalarParameterValue _returnvalue_8 "CamResY" (Math|Conversions|ToFloat(Integer) (Variables|Default|GetSensorResY)) :!class /Script/Engine.MaterialInstanceDynamic)))))
          (:then_4
            ;[1 1 1] Set main camera
            (Game|Player|SetViewTargetwithBlend (Game|GetPlayerController 0) self 0.0 "VTBlend_Linear" 0.0 false))
          (:then_5
            ;[1 1 1] Set Anim instance
            (switch Utilities|FlowControl|Switch|SwitchonESensorType (Variables|Default|GetSensorType)
              (:KINECT_V1
                (Class|SkeletalMeshComponent|SetAnimClass (Variables|Default|GetTop) "/Game/AvatarMale/K1AnimBlueprint.K1AnimBlueprint_C")
                (Class|SkeletalMeshComponent|SetAnimClass (Variables|Default|GetAvatarRaw) "/Game/AvatarMale/K1AnimBlueprintRaw.K1AnimBlueprintRaw_C"))
              (:KINECT_V2
                (Class|SkeletalMeshComponent|SetAnimClass (Variables|Default|GetTop) "/Game/AvatarMale/K2AnimBlueprint.K2AnimBlueprint_C")
                (Class|SkeletalMeshComponent|SetAnimClass (Variables|Default|GetAvatarRaw) "/Game/AvatarMale/K2AnimBlueprintRaw.K2AnimBlueprintRaw_C")))))))))

(event Input|KeyboardEvents|2
  (params (Key :type Key%20Structure))
  (bind _avataruser (Variables|Default|GetAvatarUser))
  (bind _top (Variables|Default|GetTop))
  (bind _avatarraw (Variables|Default|GetAvatarRaw))
  (bind _bottom (Variables|Default|GetBottom))
  (bind _motionsensor (Variables|Default|GetMotionSensor))
  (bind _avataruser_2 (Variables|Default|GetAvatarUser))
  ;[1 1 1] Switch between sensors
  (:Pressed
    (Development|ExecuteConsoleCommand "r.setRes 1280x720" (Game|GetPlayerController 0))
    (Variables|Default|SetSensorType "KINECT_V2")
    (Utilities|FlowControl|Sequence
      (:then_0
        (Class|MotionSensorComponent|Cleanup (Variables|Default|GetMotionSensor)))
      (:then_1
        (Variables|Default|SetOverrideSensorType false))
      (:then_2
        (Utilities|FlowControl|Sequence
          (:then_0
            ;[1 1 1] Init motion sensor
            (bind (_resx _resy _fov _widthmultiplier _returnvalue) (Class|MotionSensorComponent|Init (Variables|Default|GetMotionSensor) (Variables|Default|GetSensorType) (Variables|Default|GetOverrideSensorType)))
            ;;[1 1 1] Vertical FOV
            (Variables|Default|SetDefaultCameraFOV_Vertical _fov)
            (Variables|Default|SetSensorResX _resx)
            (Variables|Default|SetSensorResY _resy)
            (Variables|Default|SetWidthMultiplier _widthmultiplier)
            ;;[1 1 1] Could be changed with command line argument
            (Variables|Default|SetSensorType (Class|MotionSensorComponent|GetSensorType (Variables|Default|GetMotionSensor)))
            (switch Utilities|FlowControl|Switch|SwitchonESensorType (Variables|Default|GetSensorType)
              (:KINECT_V2
                ;;[1 1 1] Different value for every Kinect V2.0 sensor
                (Class|MotionSensorComponent|SetSensorOffset (Variables|Default|GetMotionSensor) "6.500000,0.000000,0.000000"))))
          (:then_1
            ;[1 1 1] Init video stream
            (if _returnvalue
              (bind _returnvalue_2 (Class|MotionSensorComponent|GetCameraFrame (Variables|Default|GetMotionSensor) "RGB"))
              (bind _returnvalue_3 (Class|MotionSensorComponent|GetCameraFrame (Variables|Default|GetMotionSensor) "USER"))
              (bind _returnvalue_4 (Class|MotionSensorComponent|CreateDynamicMaterialInstance (Variables|Default|GetMotionSensor) (Variables|Default|GetBackground) "/Game/Materials/BaseFeedScreenNoShadow.BaseFeedScreenNoShadow"))
              (Class|MotionSensorComponent|SetTextureParameterValue (Variables|Default|GetMotionSensor) _returnvalue_4 _returnvalue_2 "Color")
              (Class|MotionSensorComponent|SetTextureParameterValue (Variables|Default|GetMotionSensor) _returnvalue_4 _returnvalue_3 "NoMask")
              (Rendering|Material|SetScalarParameterValue _returnvalue_4 "CamResX" (Math|Conversions|ToFloat(Integer) (Variables|Default|GetSensorResX)) :!class /Script/Engine.MaterialInstanceDynamic)
              (Rendering|Material|SetScalarParameterValue _returnvalue_4 "CamResY" (Math|Conversions|ToFloat(Integer) (Variables|Default|GetSensorResY)) :!class /Script/Engine.MaterialInstanceDynamic)
              (bind _returnvalue_5 (Class|MotionSensorComponent|CreateDynamicMaterialInstanceSkeletal (Variables|Default|GetMotionSensor) (Variables|Default|GetAvatarUser) "/Game/Materials/Avatar.Avatar"))
              (Class|MotionSensorComponent|SetTextureParameterValue (Variables|Default|GetMotionSensor) _returnvalue_5 _returnvalue_2 "Color")
              (Class|MotionSensorComponent|SetTextureParameterValue (Variables|Default|GetMotionSensor) _returnvalue_5 "/Game/Textures/black.Black" "MaskTop")
              (Rendering|Material|SetScalarParameterValue _returnvalue_5 "CamResX" (Math|Conversions|ToFloat(Integer) (Variables|Default|GetSensorResX)) :!class /Script/Engine.MaterialInstanceDynamic)
              (Rendering|Material|SetScalarParameterValue _returnvalue_5 "CamResY" (Math|Conversions|ToFloat(Integer) (Variables|Default|GetSensorResY)) :!class /Script/Engine.MaterialInstanceDynamic)
              ;[1 1 1] User preview
              (Utilities|FlowControl|Delay 0.2)
              (bind _returnvalue_6 (Appearance|GetDynamicMaterial (Variables|/Game/UI/MainUI.MainUI_C|GetUserPreview (Variables|Default|GetUI)) :!class /Script/UMG.Image))
              (bind _returnvalue_7 (Class|MotionSensorComponent|GetCameraFrame (Variables|Default|GetMotionSensor) "USER"))
              (Rendering|Material|SetTextureParameterValue _returnvalue_6 "Color" _returnvalue_7)))
          (:then_2
            ;[1 1 1] Change gender
            (switch Utilities|FlowControl|Switch|SwitchonGender (Variables|Default|GetGender)
              (:NewEnumerator0
                (bind _output_get (Variables|Default|SetGender "NewEnumerator0"))
                (Development|PrintString (Utilities|String|EnumtoString _output_get))
                (Class|SkinnedMeshComponent|SetSkeletalMesh _avataruser "/Game/AvatarMale/MaleFitA.MaleFitA" true)
                ;;[1 1 1] Default clothing (empty, use load cloth instead of this)
                (Class|SkinnedMeshComponent|SetSkeletalMesh _top 0 true)
                (Class|SkinnedMeshComponent|SetSkeletalMesh _bottom 0 true)
                (Class|SkinnedMeshComponent|SetSkeletalMesh _avatarraw "/Game/AvatarMale/MaleFitA.MaleFitA" true))
              (:NewEnumerator1
                (bind _output_get_2 (Variables|Default|SetGender "NewEnumerator1"))
                (Development|PrintString (Utilities|String|EnumtoString _output_get_2))
                (Class|SkinnedMeshComponent|SetSkeletalMesh _avataruser "/Game/AvatarFemale/FemaleFitA.FemaleFitA" true)
                (Class|SkinnedMeshComponent|SetSkeletalMesh _top 0 true)
                (Class|SkinnedMeshComponent|SetSkeletalMesh _bottom 0 true)
                (Class|SkinnedMeshComponent|SetSkeletalMesh _avatarraw "/Game/AvatarFemale/FemaleFitA.FemaleFitA" true)))
            (if (Variables|Default|GetIsShowAvatar)
              ;[1 1 1] Avatar ON/OFF
              (switch Utilities|FlowControl|Switch|SwitchonGender (Variables|Default|GetGender)
                (:NewEnumerator0
                  (Rendering|Material|SetMaterial _avataruser_2 0 "/Game/AvatarMale/BodyMale.BodyMale"))
                (:NewEnumerator1
                  (Rendering|Material|SetMaterial _avataruser_2 0 "/Game/AvatarFemale/BodyFemale.BodyFemale")))
              (Development|PrintString "Avatar  material changed")
              (Variables|Default|SetIsShowAvatar true)))
          (:then_3
            (if _returnvalue
              (Utilities|FlowControl|Sequence
                (:then_0
                  (bind _returnvalue_8 (Class|MotionSensorComponent|CreateDynamicMaterialInstance _motionsensor (Variables|Default|GetForeGround) "/Game/Materials/DepthPreview.DepthPreview")))
                (:then_1
                  (bind _returnvalue_9 (Class|MotionSensorComponent|GetCameraFrame _motionsensor "USER")))
                (:then_2
                  (bind _returnvalue_10 (Class|MotionSensorComponent|GetCameraFrame _motionsensor "DEPTH"))
                  (Class|MotionSensorComponent|SetTextureParameterValue (Variables|Default|GetMotionSensor) _returnvalue_8 _returnvalue_2 "Color")
                  (Class|MotionSensorComponent|SetTextureParameterValue (Variables|Default|GetMotionSensor) _returnvalue_8 _returnvalue_9 "User")
                  (Class|MotionSensorComponent|SetTextureParameterValue (Variables|Default|GetMotionSensor) _returnvalue_8 _returnvalue_10 "DepthKinect")
                  (Rendering|Material|SetScalarParameterValue _returnvalue_8 "CamResX" (Math|Conversions|ToFloat(Integer) (Variables|Default|GetSensorResX)) :!class /Script/Engine.MaterialInstanceDynamic)
                  (Rendering|Material|SetScalarParameterValue _returnvalue_8 "CamResY" (Math|Conversions|ToFloat(Integer) (Variables|Default|GetSensorResY)) :!class /Script/Engine.MaterialInstanceDynamic)))))
          (:then_4
            ;[1 1 1] Set main camera
            (Game|Player|SetViewTargetwithBlend (Game|GetPlayerController 0) self 0.0 "VTBlend_Linear" 0.0 false))
          (:then_5
            ;[1 1 1] Set Anim instance
            (switch Utilities|FlowControl|Switch|SwitchonESensorType (Variables|Default|GetSensorType)
              (:KINECT_V1
                (Class|SkeletalMeshComponent|SetAnimClass (Variables|Default|GetTop) "/Game/AvatarMale/K1AnimBlueprint.K1AnimBlueprint_C")
                (Class|SkeletalMeshComponent|SetAnimClass (Variables|Default|GetAvatarRaw) "/Game/AvatarMale/K1AnimBlueprintRaw.K1AnimBlueprintRaw_C"))
              (:KINECT_V2
                (Class|SkeletalMeshComponent|SetAnimClass (Variables|Default|GetTop) "/Game/AvatarMale/K2AnimBlueprint.K2AnimBlueprint_C")
                (Class|SkeletalMeshComponent|SetAnimClass (Variables|Default|GetAvatarRaw) "/Game/AvatarMale/K2AnimBlueprintRaw.K2AnimBlueprintRaw_C")))))))))

(event Input|KeyboardEvents|Subtract
  (params (Key :type Key%20Structure))
  ;[1 1 1] Scale WIDTH
  (:Pressed
    (bind _output_get (Variables|Default|SetScaleWidthOffset (+ (Variables|Default|GetScaleWidthOffset) -0.01)))
    (Development|PrintString (Utilities|String|ToString(Float) _output_get))))

(event Input|KeyboardEvents|Add
  (params (Key :type Key%20Structure))
  ;[1 1 1] Scale WIDTH
  (:Pressed
    (bind _output_get (Variables|Default|SetScaleWidthOffset (+ (Variables|Default|GetScaleWidthOffset) 0.01)))
    (Development|PrintString (Utilities|String|ToString(Float) _output_get))))

(event Input|KeyboardEvents|G
  (params (Key :type Key%20Structure))
  (bind _avataruser (Variables|Default|GetAvatarUser))
  (bind _top (Variables|Default|GetTop))
  (bind _avatarraw (Variables|Default|GetAvatarRaw))
  (bind _bottom (Variables|Default|GetBottom))
  (bind _avataruser_2 (Variables|Default|GetAvatarUser))
  ;[1 1 1] Change gender
  (:Pressed
    (switch Utilities|FlowControl|Switch|SwitchonGender (stale Custom|GenderChange_Event Gender)
      (:NewEnumerator0
        (bind _output_get (Variables|Default|SetGender "NewEnumerator0"))
        (Development|PrintString (Utilities|String|EnumtoString _output_get))
        (Class|SkinnedMeshComponent|SetSkeletalMesh _avataruser "/Game/AvatarMale/MaleFitA.MaleFitA" true)
        ;;[1 1 1] Default clothing (empty, use load cloth instead of this)
        (Class|SkinnedMeshComponent|SetSkeletalMesh _top 0 true)
        (Class|SkinnedMeshComponent|SetSkeletalMesh _bottom 0 true)
        (Class|SkinnedMeshComponent|SetSkeletalMesh _avatarraw "/Game/AvatarMale/MaleFitA.MaleFitA" true))
      (:NewEnumerator1
        (bind _output_get_2 (Variables|Default|SetGender "NewEnumerator1"))
        (Development|PrintString (Utilities|String|EnumtoString _output_get_2))
        (Class|SkinnedMeshComponent|SetSkeletalMesh _avataruser "/Game/AvatarFemale/FemaleFitA.FemaleFitA" true)
        (Class|SkinnedMeshComponent|SetSkeletalMesh _top 0 true)
        (Class|SkinnedMeshComponent|SetSkeletalMesh _bottom 0 true)
        (Class|SkinnedMeshComponent|SetSkeletalMesh _avatarraw "/Game/AvatarFemale/FemaleFitA.FemaleFitA" true)))
    (if (Variables|Default|GetIsShowAvatar)
      ;[1 1 1] Avatar ON/OFF
      (switch Utilities|FlowControl|Switch|SwitchonGender (Variables|Default|GetGender)
        (:NewEnumerator0
          (Rendering|Material|SetMaterial _avataruser_2 0 "/Game/AvatarMale/BodyMale.BodyMale"))
        (:NewEnumerator1
          (Rendering|Material|SetMaterial _avataruser_2 0 "/Game/AvatarFemale/BodyFemale.BodyFemale")))
      (Development|PrintString "Avatar  material changed")
      (Variables|Default|SetIsShowAvatar true))))

(event Input|KeyboardEvents|A
  (params (Key :type Key%20Structure))
  (bind _avataruser (Variables|Default|GetAvatarUser))
  ;[1 1 1] Avatar ON/OFF
  (:Pressed
    (if (Variables|Default|GetIsShowAvatar)
      (Utilities|FlowControl|Sequence
        (:then_0
          ;[1 1 1] Init video stream
          (bind _returnvalue (Class|MotionSensorComponent|CreateDynamicMaterialInstanceSkeletal (Variables|Default|GetMotionSensor) (Variables|Default|GetAvatarUser) "/Game/Materials/Avatar.Avatar"))
          (Class|MotionSensorComponent|SetTextureParameterValue (Variables|Default|GetMotionSensor) _returnvalue (stale EventBeginPlay _returnvalue_2) "Color")
          (Class|MotionSensorComponent|SetTextureParameterValue (Variables|Default|GetMotionSensor) _returnvalue "/Game/Textures/black.Black" "MaskTop")
          (Rendering|Material|SetScalarParameterValue _returnvalue "CamResX" (Math|Conversions|ToFloat(Integer) (Variables|Default|GetSensorResX)) :!class /Script/Engine.MaterialInstanceDynamic)
          (Rendering|Material|SetScalarParameterValue _returnvalue "CamResY" (Math|Conversions|ToFloat(Integer) (Variables|Default|GetSensorResY)) :!class /Script/Engine.MaterialInstanceDynamic)
          ;[1 1 1] User preview
          (Utilities|FlowControl|Delay 0.2)
          (bind _returnvalue_2 (Appearance|GetDynamicMaterial (Variables|/Game/UI/MainUI.MainUI_C|GetUserPreview (Variables|Default|GetUI)) :!class /Script/UMG.Image))
          (bind _returnvalue_3 (Class|MotionSensorComponent|GetCameraFrame (Variables|Default|GetMotionSensor) "USER"))
          (Rendering|Material|SetTextureParameterValue _returnvalue_2 "Color" _returnvalue_3))
        (:then_1
          (Variables|Default|SetIsShowAvatar false)))
      (else
        (switch Utilities|FlowControl|Switch|SwitchonGender (Variables|Default|GetGender)
          (:NewEnumerator0
            (Rendering|Material|SetMaterial _avataruser 0 "/Game/AvatarMale/BodyMale.BodyMale"))
          (:NewEnumerator1
            (Rendering|Material|SetMaterial _avataruser 0 "/Game/AvatarFemale/BodyFemale.BodyFemale")))
        (Development|PrintString "Avatar  material changed")
        (Variables|Default|SetIsShowAvatar true)))))

(fn ConstructionScript
  (Variables|/Script/Engine.SceneCaptureComponent|SetShowFlagSettings (Variables|Default|GetSceneCaptureDepth) (Utilities|Array|MakeArray (Utilities|Struct|MakeEngineShowFlagsSetting "StaticMeshes") (Utilities|Struct|MakeEngineShowFlagsSetting "SkeletalMeshes" true))))

(fn DrawDebugSkeleton
  (params (Thickness :type Float%20%28single-precision%29) (Color :type Linear%20Color%20Structure))
  (bind _motionsensor (Variables|Default|GetMotionSensor))
  (bind _motionsensor_2 (Variables|Default|GetMotionSensor))
  (bind _motionsensor_3 (Variables|Default|GetMotionSensor))
  (bind _motionsensor_4 (Variables|Default|GetMotionSensor))
  (bind _motionsensor_5 (Variables|Default|GetMotionSensor))
  (bind _motionsensor_6 (Variables|Default|GetMotionSensor))
  (bind _motionsensor_7 (Variables|Default|GetMotionSensor))
  (bind _motionsensor_8 (Variables|Default|GetMotionSensor))
  (bind _motionsensor_9 (Variables|Default|GetMotionSensor))
  (bind _motionsensor_10 (Variables|Default|GetMotionSensor))
  (bind _motionsensor_11 (Variables|Default|GetMotionSensor))
  (bind _motionsensor_12 (Variables|Default|GetMotionSensor))
  (bind _motionsensor_13 (Variables|Default|GetMotionSensor))
  (bind _motionsensor_14 (Variables|Default|GetMotionSensor))
  (Variables|Default|SetThickness Thickness)
  (Variables|Default|SetColor Color)
  (Utilities|FlowControl|Sequence
    (:then_0
      ;[1 1 1] NITE SKELETON
      ;;[1 1 1] Torso
      (Rendering|Debug|DrawDebugLine (Class|MotionSensorComponent|GetBonePosition _motionsensor_2 "Head") (Class|MotionSensorComponent|GetBonePosition _motionsensor_2 "Neck") (Variables|Default|GetColor) 0.0 (Variables|Default|GetThickness))
      (Rendering|Debug|DrawDebugLine (Class|MotionSensorComponent|GetBonePosition _motionsensor_3 "Neck") (Class|MotionSensorComponent|GetBonePosition _motionsensor_3 "SpineBase") (Variables|Default|GetColor) 0.0 (Variables|Default|GetThickness))
      ;;[1 1 1] Left arm
      (Rendering|Debug|DrawDebugLine (Class|MotionSensorComponent|GetBonePosition _motionsensor_4 "Neck") (Class|MotionSensorComponent|GetBonePosition _motionsensor_4 "ShoulderLeft") (Variables|Default|GetColor) 0.0 (Variables|Default|GetThickness))
      (Rendering|Debug|DrawDebugLine (Class|MotionSensorComponent|GetBonePosition _motionsensor_5 "ShoulderLeft") (Class|MotionSensorComponent|GetBonePosition _motionsensor_5 "ElbowLeft") (Variables|Default|GetColor) 0.0 (Variables|Default|GetThickness))
      (Rendering|Debug|DrawDebugLine (Class|MotionSensorComponent|GetBonePosition _motionsensor_6 "ElbowLeft") (Class|MotionSensorComponent|GetBonePosition _motionsensor_6 "HandLeft") (Variables|Default|GetColor) 0.0 (Variables|Default|GetThickness))
      ;;[1 1 1] RightArm
      (Rendering|Debug|DrawDebugLine (Class|MotionSensorComponent|GetBonePosition _motionsensor_7 "Neck") (Class|MotionSensorComponent|GetBonePosition _motionsensor_7 "ShoulderRight") (Variables|Default|GetColor) 0.0 (Variables|Default|GetThickness))
      (Rendering|Debug|DrawDebugLine (Class|MotionSensorComponent|GetBonePosition _motionsensor_8 "ShoulderRight") (Class|MotionSensorComponent|GetBonePosition _motionsensor_8 "ElbowRight") (Variables|Default|GetColor) 0.0 (Variables|Default|GetThickness))
      (Rendering|Debug|DrawDebugLine (Class|MotionSensorComponent|GetBonePosition _motionsensor_9 "ElbowRight") (Class|MotionSensorComponent|GetBonePosition _motionsensor_9 "HandRight") (Variables|Default|GetColor) 0.0 (Variables|Default|GetThickness))
      ;;[1 1 1] Left leg
      (Rendering|Debug|DrawDebugLine (Class|MotionSensorComponent|GetBonePosition _motionsensor_10 "SpineBase") (Class|MotionSensorComponent|GetBonePosition _motionsensor_10 "HipLeft") (Variables|Default|GetColor) 0.0 (Variables|Default|GetThickness))
      (Rendering|Debug|DrawDebugLine (Class|MotionSensorComponent|GetBonePosition _motionsensor_11 "HipLeft") (Class|MotionSensorComponent|GetBonePosition _motionsensor_11 "KneeLeft") (Variables|Default|GetColor) 0.0 (Variables|Default|GetThickness))
      (Rendering|Debug|DrawDebugLine (Class|MotionSensorComponent|GetBonePosition _motionsensor_12 "KneeLeft") (Class|MotionSensorComponent|GetBonePosition _motionsensor_12 "FootLeft") (Variables|Default|GetColor) 0.0 (Variables|Default|GetThickness))
      ;;[1 1 1] Left leg
      (Rendering|Debug|DrawDebugLine (Class|MotionSensorComponent|GetBonePosition _motionsensor_13 "SpineBase") (Class|MotionSensorComponent|GetBonePosition _motionsensor_13 "HipRight") (Variables|Default|GetColor) 0.0 (Variables|Default|GetThickness))
      (Rendering|Debug|DrawDebugLine (Class|MotionSensorComponent|GetBonePosition _motionsensor_14 "HipRight") (Class|MotionSensorComponent|GetBonePosition _motionsensor_14 "KneeRight") (Variables|Default|GetColor) 0.0 (Variables|Default|GetThickness))
      (Rendering|Debug|DrawDebugLine (Class|MotionSensorComponent|GetBonePosition _motionsensor "KneeRight") (Class|MotionSensorComponent|GetBonePosition _motionsensor "FootRight") (Variables|Default|GetColor) 0.0 (Variables|Default|GetThickness)))))

(fn GetBodyOffset
  (params (Verbose :type Boolean))
  (bind _motionsensor (Variables|Default|GetMotionSensor))
  (bind _avatarraw (Variables|Default|GetAvatarRaw))
  (return (- (/ (+ (Class|MotionSensorComponent|GetBonePosition _motionsensor "HipLeft") (Class|MotionSensorComponent|GetBonePosition _motionsensor "HipRight")) 2.0) (/ (+ (Transformation|GetSocketLocation _avatarraw "thigh_l") (Transformation|GetSocketLocation _avatarraw "thigh_r")) 2.0)) (- (Class|MotionSensorComponent|GetBonePosition (Variables|Default|GetMotionSensor) "Neck") (/ (+ (Transformation|GetSocketLocation _avatarraw "upperarm_l") (Transformation|GetSocketLocation _avatarraw "upperarm_r")) 2.0))))

(fn SetAnimOffset
  (params (SkeletalMesh :type Skeletal%20Mesh%20Component%20Object%20Reference) (OffsetVectorHip :type Vector) (OffsetVectorNeck :type Vector) (ScaleWidth :type Float%20%28single-precision%29))
  (bind _askinect_anim_instance (Utilities|Casting|CastToKinectAnimInstance (Components|SkeletalMesh|GetAnimInstance SkeletalMesh)))
  (Variables|/Script/VirtualMirrorPlugin.KinectAnimInstance|SetOffsetVectorHip _askinect_anim_instance OffsetVectorHip)
  (Variables|/Script/VirtualMirrorPlugin.KinectAnimInstance|SetOffsetVectorNeck _askinect_anim_instance OffsetVectorNeck)
  (Variables|/Script/VirtualMirrorPlugin.KinectAnimInstance|SetScaleWidth _askinect_anim_instance ScaleWidth)
  (switch Utilities|FlowControl|Switch|SwitchonGender (Variables|Default|GetGender)
    (:NewEnumerator0
      (Variables|/Script/VirtualMirrorPlugin.KinectAnimInstance|SetFootOffset _askinect_anim_instance 0.0)
      ;[1 1 1] Not using anymore
      (Variables|/Script/VirtualMirrorPlugin.KinectAnimInstance|SetPelvisOffset _askinect_anim_instance 0.0))
    (:NewEnumerator1
      (Variables|/Script/VirtualMirrorPlugin.KinectAnimInstance|SetFootOffset _askinect_anim_instance 5.0)
      (Variables|/Script/VirtualMirrorPlugin.KinectAnimInstance|SetPelvisOffset _askinect_anim_instance -3.0))))

(fn GetBodyScale
  (bind _motionsensor (Variables|Default|GetMotionSensor))
  (bind _motionsensor_2 (Variables|Default|GetMotionSensor))
  (bind _avatarraw (Variables|Default|GetAvatarRaw))
  (return (/ (Math|Vector|VectorLength (- (Class|MotionSensorComponent|GetBonePosition _motionsensor "ShoulderLeft") (Class|MotionSensorComponent|GetBonePosition _motionsensor "ShoulderRight"))) (Math|Vector|VectorLength (- (Transformation|GetSocketLocation _avatarraw "upperarm_l") (Transformation|GetSocketLocation _avatarraw "upperarm_r")))) (/ (Math|Vector|VectorLength (- (Class|MotionSensorComponent|GetBonePosition _motionsensor_2 "HipLeft") (Class|MotionSensorComponent|GetBonePosition _motionsensor_2 "HipRight"))) (Math|Vector|VectorLength (- (Transformation|GetSocketLocation _avatarraw "thigh_l") (Transformation|GetSocketLocation _avatarraw "thigh_r"))))))

(fn SetOcclusionMap
  (params (TargetComponent :type Skeletal%20Mesh%20Component%20Object%20Reference) (OcclusionTexture :type Texture%202D%20Object%20Reference) (FullBody :type Boolean))
  (bind _returnvalue (Utilities|GetDisplayName TargetComponent))
  (bind _asmaterial_instance_dynamic (Utilities|Casting|CastToMaterialInstanceDynamic (Rendering|Material|GetMaterial (Variables|Default|GetAvatarUser) 0))
    (:then
      ;[1 1 1] If fullbody reset all target nodes
      (if FullBody
        (Rendering|Material|SetTextureParameterValue _asmaterial_instance_dynamic "MaskTop" "/Game/Textures/White.White")
        (Rendering|Material|SetTextureParameterValue _asmaterial_instance_dynamic "MaskBottom" "/Game/Textures/White.White")
        (Development|PrintString "Top and Bottom occlusion textures reseted"))
      (if (Utilities|Enum|Equal(Enum) (Utilities|GetDisplayName (Variables|Default|GetTop)) _returnvalue)
        (Rendering|Material|SetTextureParameterValue _asmaterial_instance_dynamic "MaskTop" OcclusionTexture)
        (Development|PrintString "Top occlusion texture applied")
        (elif (Utilities|Enum|Equal(Enum) _returnvalue (Utilities|GetDisplayName (Variables|Default|GetBottom)))
          (Rendering|Material|SetTextureParameterValue _asmaterial_instance_dynamic "MaskBottom" OcclusionTexture)
          (Development|PrintString "Bottom occlusion texture applied"))))
    (:CastFailed
      (Development|PrintString "Cast failed"))))